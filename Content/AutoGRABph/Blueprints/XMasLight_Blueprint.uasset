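; Blueprint that strings Christmas lights along a spline when play begins.
; It spawns XMasLight actors at fixed Spacing intervals along the spline's length, each scaled down and randomly rotated.
; A wrapping counter cycles through ListOfColors to set each light's Bulb material, producing a repeating color sequence.
; The construction script is empty, so the lights are created only at runtime.
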(event EventBeginPlay
  (bind _spline (Variables|Default|GetSpline))
  (bind _listofcolors (Variables|Default|GetListOfColors))
  (for _index (range 0 (.ReturnValue (Math|Float|Division(WholeandRemainder) (Spline|GetSplineLength _spline) (Variables|Default|GetSpacing))))
    (bind _returnvalue (Game|SpawnActorfromClass "/Game/AutoGRABph/Blueprints/XMasLight.XMasLight_C" (Math|Transform|MakeTransform (Spline|GetLocationatDistanceAlongSpline _spline (* _index (Variables|Default|GetSpacing)) "World") (Math|Rotator|MakeRotator (Math|Random|RandomFloatinRange 0.0 3.6e+02) (Math|Random|RandomFloatinRange 0.0 3.6e+02) (Math|Random|RandomFloatinRange 0.0 3.6e+02)) "0.050000,0.050000,0.050000") "Undefined" 0 0))
    (bind _result (Math|Integer|IncrementInt (Variables|Default|GetLoop))
      (:%20%20
        (bind _output_get (Variables|Default|SetLoop _result))
        (if (>= _output_get (Utilities|Array|Length _listofcolors))
          (Variables|Default|SetLoop 0))
        (Rendering|Material|SetMaterial (Variables|/Game/AutoGRABph/Blueprints/XMasLight.XMasLight_C|GetBulb _returnvalue) 0 (Utilities|Array|Get(acopy) _listofcolors (Variables|Default|GetLoop)))))))

(event Collision|EventActorBeginOverlap
  (params (OtherActor :type Actor%20Object%20Reference)))

(event EventTick
  (params (DeltaSeconds :type Float%20%28single-precision%29)))

(fn ConstructionScript)