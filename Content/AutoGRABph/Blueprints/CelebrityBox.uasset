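; CelebrityBox is a celebrity NPC trigger that shows the name and flags the first-person character's AIOverlap while overlapped.
; Externally triggered talk events display the current DialogueLines entry in AIDialogueWidget, colored by speaker, with an optional scribble sound.
; Tobey has separate no-knife and with-knife events that split one line array at index 4.
; Leaving mid-conversation hides the widget and resets the line index if dialogue is unfinished.
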(event OnComponentBeginOverlap(Box)
  (params (OverlappedComponent :type Primitive%20Component%20Object%20Reference) (OtherActor :type Actor%20Object%20Reference) (OtherComp :type Primitive%20Component%20Object%20Reference) (OtherBodyIndex :type Integer) (bFromSweep :type Boolean) (SweepResult :type Hit%20Result%20Structure%20%28by%20ref%29))
  ;[1 1 1] Overlap Logic
  (bind _asfirst_person_character (Utilities|Casting|CastToFirstPersonCharacter OtherActor))
  (Rendering|Components|TextRender|SetText (Variables|Default|GetTextRender) (Variables|Default|GetCelebrityName))
  (Variables|/Game/FirstPersonBP/Blueprints/FirstPersonCharacter.FirstPersonCharacter_C|SetAIOverlap _asfirst_person_character true))

(event OnComponentEndOverlap(Box)
  (params (OverlappedComponent :type Primitive%20Component%20Object%20Reference) (OtherActor :type Actor%20Object%20Reference) (OtherComp :type Primitive%20Component%20Object%20Reference) (OtherBodyIndex :type Integer))
  ;[1 1 1] Overlap Logic
  (bind _asfirst_person_character (Utilities|Casting|CastToFirstPersonCharacter OtherActor))
  (Rendering|Components|TextRender|SetText (Variables|Default|GetTextRender) (Utilities|Text|MakeLiteralText ""))
  (Variables|/Game/FirstPersonBP/Blueprints/FirstPersonCharacter.FirstPersonCharacter_C|SetAIOverlap _asfirst_person_character false)
  (if (Variables|Default|GetIsTalking)
    (Variables|Default|SetIsTalking false)
    (if (Variables|Default|GetIsTobey)
      (if (Variables|Default|GetStartedTobeyKnifeConvo?)
        (Widget|SetVisibility (stale Custom|TobeyWithKnife%20Talk%20Event _array_element) "Hidden")
        (if (Variables|Default|GetFinishedDialogue)
          (Variables|Default|SetStartedTobeyKnifeConvo? true)
          (else
            (Variables|Default|SetStartedTobeyKnifeConvo? false)))
        (else
          (Widget|SetVisibility (stale Custom|TobeyNoKnife%20Talk%20Eve _array_element) "Hidden")))
      (else
        (Widget|SetVisibility (stale Custom|Talk%20Event _array_element) "Hidden")))
    (if (not (Variables|Default|GetFinishedDialogue))
      (Variables|Default|SetDialogueLineNum 0))))

(event Custom|TobeyWithKnife%20Talk%20Event
  ;[1 1 1] Tobey With Knife Dialogue
  (if (Variables|Default|GetStartedTobeyKnifeConvo?)
    _
    (else
      (Variables|Default|SetStartedTobeyKnifeConvo? true)
      (Variables|Default|SetFinishedDialogue false)
      (Variables|Default|SetDialogueLineNum 4)))
  (bind _foundwidgets (Widget|GetAllWidgetsOfClass "/Game/AutoGRABph/Blueprints/AIDialogueWidget.AIDialogueWidget_C" true))
  (for _array_element _foundwidgets
    (if (<= (Variables|Default|GetDialogueLineNum) (- (Utilities|Array|Length (Variables|Default|GetDialogueLines)) 1))
      (Variables|/Game/AutoGRABph/Blueprints/AIDialogueWidget.AIDialogueWidget_C|SetDialogue _array_element (Utilities|Array|Get(acopy) (Variables|Default|GetDialogueLines) (Variables|Default|GetDialogueLineNum)))
      (Widget|SetVisibility _array_element "Visible")
      (if (== (Variables|Default|GetDialogueLineNum) (Variables|Default|GetScribbleSoundIndex))
        (Audio|Components|Audio|Play (Variables|Default|Getoffice_writing_scribbling_ballpoint_pen_on_paper_0_Cue) 0.0))
      ;[1 1 1] If NPC is talking for a particular line, set the color to NPCTextColor, else just set it to white
      (if (Utilities|Array|Get(acopy) (Variables|Default|GetIsNPCTalking) (Variables|Default|GetDialogueLineNum))
        (Variables|/Game/AutoGRABph/Blueprints/AIDialogueWidget.AIDialogueWidget_C|SetColor _array_element (Variables|Default|GetNPCTextColor))
        (else
          (Variables|/Game/AutoGRABph/Blueprints/AIDialogueWidget.AIDialogueWidget_C|SetColor _array_element (Math|Conversions|ToColor(LinearColor) "(R=1.000000,G=1.000000,B=1.000000,A=1.000000)"))))
      (else
        (Widget|SetVisibility _array_element "Hidden")
        (Variables|Default|SetFinishedDialogue true)))))

(event Custom|Talk%20Event
  (bind _dialoguelinenum (Variables|Default|GetDialogueLineNum))
  ;[1 1 1] Dialogue Logic
  (bind _foundwidgets (Widget|GetAllWidgetsOfClass "/Game/AutoGRABph/Blueprints/AIDialogueWidget.AIDialogueWidget_C" true))
  (for _array_element _foundwidgets
    (if (<= _dialoguelinenum (- (Utilities|Array|Length (Variables|Default|GetDialogueLines)) 1))
      (Variables|/Game/AutoGRABph/Blueprints/AIDialogueWidget.AIDialogueWidget_C|SetDialogue _array_element (Utilities|Array|Get(acopy) (Variables|Default|GetDialogueLines) _dialoguelinenum))
      (Widget|SetVisibility _array_element "Visible")
      (if (== _dialoguelinenum (Variables|Default|GetScribbleSoundIndex))
        (Audio|Components|Audio|Play (Variables|Default|Getoffice_writing_scribbling_ballpoint_pen_on_paper_0_Cue) 0.0))
      ;[1 1 1] If NPC is talking for a particular line, set the color to NPCTextColor, else just set it to white
      (if (Utilities|Array|Get(acopy) (Variables|Default|GetIsNPCTalking) _dialoguelinenum)
        (Variables|/Game/AutoGRABph/Blueprints/AIDialogueWidget.AIDialogueWidget_C|SetColor _array_element (Variables|Default|GetNPCTextColor))
        (else
          (Variables|/Game/AutoGRABph/Blueprints/AIDialogueWidget.AIDialogueWidget_C|SetColor _array_element (Math|Conversions|ToColor(LinearColor) "(R=1.000000,G=1.000000,B=1.000000,A=1.000000)"))))
      (else
        (Widget|SetVisibility _array_element "Hidden")
        (Variables|Default|SetFinishedDialogue true)))))

(event Custom|TobeyNoKnife%20Talk%20Eve
  (bind _dialoguelinenum (Variables|Default|GetDialogueLineNum))
  ;[1 1 1] Tobey No Knife Dialogue
  (bind _foundwidgets (Widget|GetAllWidgetsOfClass "/Game/AutoGRABph/Blueprints/AIDialogueWidget.AIDialogueWidget_C" true))
  (for _array_element _foundwidgets
    (if (<= _dialoguelinenum 3)
      (Variables|/Game/AutoGRABph/Blueprints/AIDialogueWidget.AIDialogueWidget_C|SetDialogue _array_element (Utilities|Array|Get(acopy) (Variables|Default|GetDialogueLines) _dialoguelinenum))
      (Widget|SetVisibility _array_element "Visible")
      ;[1 1 1] If NPC is talking for a particular line, set the color to NPCTextColor, else just set it to white
      (if (Utilities|Array|Get(acopy) (Variables|Default|GetIsNPCTalking) _dialoguelinenum)
        (Variables|/Game/AutoGRABph/Blueprints/AIDialogueWidget.AIDialogueWidget_C|SetColor _array_element (Variables|Default|GetNPCTextColor))
        (else
          (Variables|/Game/AutoGRABph/Blueprints/AIDialogueWidget.AIDialogueWidget_C|SetColor _array_element (Math|Conversions|ToColor(LinearColor) "(R=1.000000,G=1.000000,B=1.000000,A=1.000000)"))))
      (else
        (Widget|SetVisibility _array_element "Hidden")
        (Variables|Default|SetFinishedDialogue true)))))

(event EventBeginPlay
  (Rendering|Components|TextRender|SetText (Variables|Default|GetTextRender) (Utilities|Text|MakeLiteralText "")))

(event Collision|EventActorBeginOverlap
  (params (OtherActor :type Actor%20Object%20Reference)))

(event EventTick
  (params (DeltaSeconds :type Float%20%28single-precision%29)))

(fn ConstructionScript)